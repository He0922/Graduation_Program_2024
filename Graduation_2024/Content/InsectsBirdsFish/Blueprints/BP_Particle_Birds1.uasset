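; Configurable particle actor for bird effects, with an optional repeating burst mode.
; The construction script assigns the particle template and feeds spawn amount, radius, size, lifetime and speed into its named parameters.
; When BurstEffect is on, BeginPlay activates the particle, waits out the lifetime plus a retrigger delay, then loops through the SpawnBirds event to activate it again.
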(event `self.ReceiveBeginPlay`
  ;[1 1 1] TriggerBurstBirds
  (if (`self.BurstEffect`) :!label _label
    (`ActorComponent.Activate` (`self.Particle`) false)
    (`KismetSystemLibrary.Delay` (`self.Lifetime`))
    (`KismetSystemLibrary.Delay` (`self.RetriggerTime`))
    (`self.SpawnBirds`)))

(event `SpawnBirds`
  ;[1 1 1] TriggerBurstBirds
  (goto _label))

(fn `UserConstructionScript`
  (bind _particle (`self.Particle`))
  ;[1 1 1] Initial Setup
  (`ParticleSystemComponent.SetTemplate` (`self.Particle`) (`self.ParticleTemplate`))
  (`ParticleSystemComponent.SetFloatParameter` _particle "Spawn" (`self.SpawnAmount`))
  (`ParticleSystemComponent.SetFloatParameter` _particle "Radius" (`self.SpawnRadius`))
  (`ParticleSystemComponent.SetVectorParameter` _particle "Size" (`KismetMathLibrary.Conv_DoubleToVector` (`self.ParticleSize`)))
  (`ParticleSystemComponent.SetFloatParameter` _particle "Lifetime" (`self.Lifetime`))
  (`ParticleSystemComponent.SetVectorParameter` _particle "Speed" (`KismetMathLibrary.Conv_DoubleToVector` (`self.Speed`))))