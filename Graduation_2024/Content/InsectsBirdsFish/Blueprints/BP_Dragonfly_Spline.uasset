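; Ambient dragonfly actor that moves a particle effect between the points of a spline in an endless circuit.
; The construction script applies the template and places it at a configurable starting point and scale.
; After each random delay, a timeline lerps it to the next point, with random position and rotation offsets and one of three randomly chosen easing tracks.
; Each arrival becomes the next start, wrapping at the spline's end.
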(event `Loop`
  (bind (_returnvalue_location _returnvalue_rotation) (`KismetMathLibrary.BreakTransform` (`KismetMathLibrary.TLerp` (`self.StartPoint`) (`self.EndPoint`) (`self.Lerp`))))
  (bind _returnvalue (+ (`self.CurrentSplinePoint`) 1))
  (bind (_returnvalue_location_2 _returnvalue_rotation_2 _returnvalue_scale) (`KismetMathLibrary.BreakTransform` (`SplineComponent.GetTransformAtSplinePoint` (`self.Spline`) (`KismetMathLibrary.SelectInt` 0 _returnvalue (> _returnvalue (`self.NumberOfPoints`))) "Local" false)))
  ;[1 1 1] Delay Loop
  (`KismetSystemLibrary.Delay` (`KismetMathLibrary.RandomFloatInRange` (`self.Delay_Min`) (`self.Delay_Max`)) :!label _label)
  ;[1 1 1] Randomiser
  (set `self.Randomiser` (`KismetMathLibrary.RandomIntegerInRange` 0 2))
  (set `self.EndPoint` (`KismetMathLibrary.MakeTransform` (+ _returnvalue_location_2 (* (`KismetMathLibrary.RandomUnitVector`) (`self.Random_Offset`))) (`KismetMathLibrary.ComposeRotators` _returnvalue_rotation_2 (* (`KismetMathLibrary.RandomRotator` false) (`self.Random_Rotation`))) _returnvalue_scale))
  ;[1 1 1] Fly From Point to Point
  (bind (_direction _lerp _lerp1 _lerp2) (`Timeline|Fly` :!via `PlayFromStart`)
    (:`Update`
      (switch `int` (`self.Randomiser`)
        (:`0`
          (set `self.Lerp` _lerp))
        (:`1`
          (set `self.Lerp` _lerp1))
        (:`2`
          (set `self.Lerp` _lerp2)))
      (`SceneComponent.K2_SetRelativeTransform` (`self.P_Dragonfly`) (`KismetMathLibrary.MakeTransform` _returnvalue_location _returnvalue_rotation (`KismetMathLibrary.Conv_DoubleToVector` (`self.Scale`))) false false))
    (:`Finished`
      ;[1 1 1] Increment Point
      (set `self.StartPoint` (`self.EndPoint`))
      (bind _result (`/Engine/EditorBlueprintResources/StandardMacros.IncrementInt` (`self.CurrentSplinePoint`))
        (:`  `
          (if (> _result (`self.NumberOfPoints`))
            (set `self.CurrentSplinePoint` 0))
          (`self.Loop`))))))

(event `self.ReceiveBeginPlay`
  ;[1 1 1] Delay Loop
  (goto _label))

(fn `UserConstructionScript`
  ;[1 1 1] Set Starting Point and Scale
  (`ParticleSystemComponent.SetTemplate` (`self.P_Dragonfly`) (`self.Template`))
  (set `self.NumberOfPoints` (`SplineComponent.GetNumberOfSplinePoints` (`self.Spline`)))
  (bind _output_get (set `self.CurrentSplinePoint` (mod (`self.Starting_Point`) (`self.NumberOfPoints`))))
  (bind (_returnvalue_location _returnvalue_rotation) (`KismetMathLibrary.BreakTransform` (`SplineComponent.GetTransformAtSplinePoint` (`self.Spline`) _output_get "Local" false)))
  (bind _output_get_2 (set `self.StartPoint` (`KismetMathLibrary.MakeTransform` _returnvalue_location _returnvalue_rotation (`KismetMathLibrary.Conv_DoubleToVector` (`self.Scale`)))))
  (`SceneComponent.K2_SetRelativeTransform` (`self.P_Dragonfly`) _output_get_2 false false))