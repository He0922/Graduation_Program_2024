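; BP_Particle_Swarm is a configurable particle swarm actor that can travel along a spline, apparently for ambient insects, birds or fish.
; The construction script applies the chosen particle template, feeds in spawn amount, radius and size parameters, and places the emitter at its starting spline position when animation is enabled.
; At BeginPlay, a timeline moves the emitter by spline distance, using the fractional part of scaled time plus start offset to wrap laps.
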(event `self.ReceiveBeginPlay`
  (bind _spline (`self.Spline`))
  ;[1 1 1] Loop Along Spline
  (if (`self.AnimateAlongSpline`)
    (bind (_direction _lerp) (`Timeline|Loop`)
      (:`Update`
        (`SceneComponent.K2_SetRelativeLocation` (`self.Particle`) (`SplineComponent.GetLocationAtDistanceAlongSpline` _spline (* (`SplineComponent.GetSplineLength` _spline) (`KismetMathLibrary.Fraction` (+ (* (`self.LoopsPerMinute`) _lerp) (`self.StartingPosition`)))) "Local") false false)))))

(fn `UserConstructionScript`
  (bind _particle (`self.Particle`))
  (bind _spline (`self.Spline`))
  ;[1 1 1] Initial Setup
  (`ParticleSystemComponent.SetTemplate` (`self.Particle`) (`self.ParticleTemplate`))
  (`ParticleSystemComponent.SetFloatParameter` _particle "Spawn" (`self.SpawnAmount`))
  (`ParticleSystemComponent.SetFloatParameter` _particle "Radius" (`self.SpawnRadius`))
  (`ParticleSystemComponent.SetFloatParameter` _particle "Size" (`self.ParticleSize`))
  (if (`self.AnimateAlongSpline`)
    (`SceneComponent.K2_SetRelativeLocation` (`self.Particle`) (`SplineComponent.GetLocationAtDistanceAlongSpline` _spline (* (`SplineComponent.GetSplineLength` _spline) (`KismetMathLibrary.Fraction` (`self.StartingPosition`))) "Local") false false)))