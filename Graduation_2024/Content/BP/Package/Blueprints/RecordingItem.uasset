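; RecordingItem is a Blueprint that displays a given static mesh and can spin it, apparently as a model for recording through its Camera component.
; InitRecordingItem assigns the mesh and zeroes its relative rotation, while BeginPlay resets the Camera's post-process settings.
; Start and end rotation events toggle a flag and set the speed, which Tick uses for frame-rate-independent local yaw.
; CloseLight and the construction script are empty.
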(event `self.ReceiveBeginPlay`
  (set `CameraComponent.PostProcessSettings` (struct) (`self.Camera`)))

(event `InitRecordingItem`
  (params (Mesh :type "StaticMesh Object Reference"))
  (`StaticMeshComponent.SetStaticMesh` (`self.StaticMesh`) Mesh)
  (`SceneComponent.K2_SetRelativeRotation` :`self` (`self.StaticMesh`)))

(event `SatrtRotate Model`
  (params (Rotation :type "Float (double-precision)"))
  (set `self.CanRotate` true)
  (set `self.RotationSpeed` Rotation))

(event `EndRotate`
  (set `self.CanRotate` false))

(event `self.ReceiveTick`
  (params (DeltaSeconds :type "Float (single-precision)"))
  (if (`self.CanRotate`)
    (`SceneComponent.K2_AddLocalRotation` (`self.StaticMesh`) (`KismetMathLibrary.MakeRotator` 0.0 0.0 (* DeltaSeconds (`self.RotationSpeed`))) false false)))

(fn `CloseLight`)

(fn `UserConstructionScript`)