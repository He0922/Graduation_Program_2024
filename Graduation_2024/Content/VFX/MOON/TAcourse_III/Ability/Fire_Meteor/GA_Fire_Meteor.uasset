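; Fire Meteor ability that calls a meteor down on the player's cursor location when the ability key is released.
; If the cooldown check allows it, the release applies the cooldown and spawns GE_Meteor and GE_MeteorRune.
; The meteor's override transform starts at a random point in an upward cone above the cursor, offset by DistanceToTarget, with a look-at rotation toward the cursor.
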(event `self.CE_KeyReleased`
  (bind (_cursordata_bblockinghit _cursordata_binitialoverlap _cursordata_time _cursordata_distance _cursordata_location) (`GameplayStatics.BreakHitResult` (`/Game/VFX/MOON/TAcourse_III/GameBP/Pawn/Player/B_ElementalPlayer.CursorData` (`self.ElementalPlayer`))))
  (bind _returnvalue (+ _cursordata_location (* (`KismetMathLibrary.RandomUnitVectorInConeInDegrees` (0.0 0.0 1.0) 45.0) (`self.DistanceToTarget`))))
  ;[1 1 1] 默认情况下, 松开按键视为 cast 技能 并检查和设置CD
  (bind _cd (`self.CF_CdCheck`))
  (if (not _cd)
    (`self.CF_ApplyCd`)
    (`self.SpawnGE` "/Game/VFX/MOON/TAcourse_III/Ability/Fire_Meteor/GE_Meteor.GE_Meteor_C" (`KismetMathLibrary.MakeTransform` _returnvalue (`KismetMathLibrary.FindLookAtRotation` _returnvalue _cursordata_location)) true true)
    (`self.SpawnGE` "/Game/VFX/MOON/TAcourse_III/Ability/Fire_Meteor/GE_MeteorRune.GE_MeteorRune_C")))

(fn `UserConstructionScript`
  (`parent.UserConstructionScript`))