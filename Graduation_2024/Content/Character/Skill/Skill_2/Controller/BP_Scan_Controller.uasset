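; Player controller component for the scan skill, fading a post-process scan effect in and out.
; StartScan and EndScan drive a fade state machine, with Tick advancing normalized time at separate in/out speeds.
; During fades it feeds time and pawn location to material parameters and sets blend weight, optionally curve-remapped.
; BP_ScanActor is spawned lazily with a dynamic post-process material; fully fading out disables tick and optionally destroys it.
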(event `self.ReceiveBeginPlay`
  (bind `_as玩家控制器` (cast `PlayerController` (`self.GetOwner`))
    (:`then`
      (set `self.Player Controller` `_as玩家控制器`)
      (`self.UpdateScanState` "NewEnumerator3" true)
      (`KismetMaterialLibrary.SetScalarParameterValue` null "Range" (`self.Range`))
      (`KismetMaterialLibrary.SetScalarParameterValue` null "GridCellSize" (`self.GridCellSize`)))
    (:`CastFailed`
      (`self.UpdateScanState` "NewEnumerator4" true))))

(event `self.ReceiveTick`
  (params (DeltaSeconds :type "Float (single-precision)"))
  (bind _player_controller (`self.Player Controller`))
  (bind _returnvalue (`Controller.K2_GetPawn` _player_controller))
  (`self.UpdateScanTime` DeltaSeconds)
  (switch `/Game/Character/Skill/Skill_2/Controller/EBP_ScanState` (`self.GetScanState`)
    (:`NewEnumerator0`
      _)
    (:`NewEnumerator2`
      _))
  (`self.UpdateScanPPBlendWeight`)
  (`/Engine/EditorBlueprintResources/StandardMacros.IsValid` _player_controller
    (:`Is Valid`
      (`/Engine/EditorBlueprintResources/StandardMacros.IsValid` _returnvalue
        (:`Is Valid`
          (`KismetMaterialLibrary.SetVectorParameterValue` null "Location" (`KismetMathLibrary.Conv_VectorToLinearColor` (`Actor.K2_GetActorLocation` _returnvalue))))))))

(fn `DestroyPPActor`
  (bind _scanactor (`self.ScanActor`))
  (if (and (`KismetSystemLibrary.IsValid` _scanactor) (`self.bDestroyActor`))
    (`Actor.K2_DestroyActor` _scanactor)
    (set `self.ScanActor` null)))

(fn `End Scan`
  (switch `/Game/Character/Skill/Skill_2/Controller/EBP_ScanState` (`self.GetScanState`)
    (:`NewEnumerator0`
      _)
    (:`NewEnumerator1`
      _)
    (:`NewEnumerator2`
      (return))
    (:`NewEnumerator3`
      (return))
    (:`NewEnumerator4`
      (return)))
  (`self.UpdateScanState` "NewEnumerator2")
  (return))

(fn `GetScanPPActor`
  (returns (`Scan Actor` :type "/Game/Character/Skill/Skill_2/BP_ScanActor Object Reference"))
  (bind _pp_material (`self.PP Material`))
  (bind _postprocess (`/Game/Character/Skill/Skill_2/BP_ScanActor.PostProcess` (`self.ScanActor`)))
  (`/Engine/EditorBlueprintResources/StandardMacros.IsValid` (`self.ScanActor`)
    (:`Is Valid`
      (return (stale _output_get)))
    (:`Is Not Valid`
      (bind _returnvalue (`|SpawnActorFromClass` "/Game/Character/Skill/Skill_2/BP_ScanActor.BP_ScanActor_C" (`KismetMathLibrary.MakeTransform` (0.0 0.0 0.0)) "Undefined" "MultiplyWithRoot" null null))
      (bind _output_get (set `self.ScanActor` _returnvalue))
      (`|ExecutionSequence`
        (:`then_0`
          (`/Engine/EditorBlueprintResources/StandardMacros.IsValid` (`self.PP MID`)
            (:`Is Valid`
              _)
            (:`Is Not Valid`
              (`/Engine/EditorBlueprintResources/StandardMacros.IsValid` _pp_material
                (:`Is Valid`
                  (bind _returnvalue_2 (`KismetMaterialLibrary.CreateDynamicMaterialInstance` _pp_material))
                  (bind _output_get_2 (set `self.PP MID` _returnvalue_2))))))
          (`/Engine/EditorBlueprintResources/StandardMacros.IsValid` _postprocess
            (:`Is Valid`
              (setmembers `PostProcessSettings` :`StructRef` (`PostProcessComponent.Settings` _postprocess) :`WeightedBlendables` (make `WeightedBlendables` (`|MakeArray` (make `WeightedBlendable` 1.0 (`self.PP MID`))))))))
        (:`then_1`
          (return _output_get))))))

(fn `GetScanState`
  (returns (State :type "/Game/Character/Skill/Skill_2/Controller/EBP_ScanState Enum"))
  (return (`self.State`)))

(fn `StartScan`
  (switch `/Game/Character/Skill/Skill_2/Controller/EBP_ScanState` (`self.GetScanState`)
    (:`NewEnumerator0`
      _)
    (:`NewEnumerator1`
      _)
    (:`NewEnumerator2`
      (`self.UpdateScanState` "NewEnumerator0" :!label _label)
      (return))
    (:`NewEnumerator3`
      (goto _label))
    (:`NewEnumerator4`
      _))
  (return))

(fn `UpdateScanPPBlendWeight`
  (locals (`This Time` :type "Float (single-precision)" :default 0.0))
  (bind _blendcurve (`self.BlendCurve`))
  (bind _scannormailzedtime (`self.ScanNormailzedTime`))
  (`/Engine/EditorBlueprintResources/StandardMacros.IsValid` _blendcurve
    (:`Is Valid`
      (set `local.This Time` (`CurveFloat.GetFloatValue` _blendcurve _scannormailzedtime)))
    (:`Is Not Valid`
      (set `local.This Time` _scannormailzedtime)))
  (bind _scan_actor (`self.GetScanPPActor`))
  (`/Engine/EditorBlueprintResources/StandardMacros.IsValid` _scan_actor
    (:`Is Valid`
      (bind _postprocess (`/Game/Character/Skill/Skill_2/BP_ScanActor.PostProcess` _scan_actor))
      (`/Engine/EditorBlueprintResources/StandardMacros.IsValid` _postprocess
        (:`Is Valid`
          (set `PostProcessComponent.BlendWeight` (`local.This Time`) _postprocess))))))

(fn `UpdateScanState`
  (params (State :type "/Game/Character/Skill/Skill_2/Controller/EBP_ScanState Enum" :default "NewEnumerator0") (Force :type Boolean))
  (returns (Update :type Boolean))
  (if (or Force (`|EnumInequality` State (`self.State`)))
    (`|ExecutionSequence`
      (:`then_0`
        (switch `/Game/Character/Skill/Skill_2/Controller/EBP_ScanState` (`self.State`)
          (:`NewEnumerator1`
            (`KismetMaterialLibrary.SetScalarParameterValue` null "bFadeIn"))
          (:`NewEnumerator3`
            (`KismetMaterialLibrary.SetScalarParameterValue` null "bFadeOut")
            (`self.SetComponentTickEnabled` true))))
      (:`then_1`
        (bind _output_get (set `self.State` State))
        (switch `/Game/Character/Skill/Skill_2/Controller/EBP_ScanState` _output_get
          (:`NewEnumerator1`
            (`KismetMaterialLibrary.SetScalarParameterValue` null "bFadeIn")
            (`self.UpdateScanPPBlendWeight`))
          (:`NewEnumerator3`
            (`KismetMaterialLibrary.SetScalarParameterValue` null "bFadeOut")
            (`self.UpdateScanPPBlendWeight`)
            (`self.SetComponentTickEnabled` false :!label _label)
            (`self.DestroyPPActor`))
          (:`NewEnumerator4`
            (goto _label))))
      (:`then_2`
        (return true)))
    (else
      (return false))))

(fn `UpdateScanTime`
  (params (DeltaTime :type "Float (double-precision)"))
  (returns (bUpdated :type Boolean))
  (`|ExecutionSequence`
    (:`then_0`
      (switch `/Game/Character/Skill/Skill_2/Controller/EBP_ScanState` (`self.GetScanState`)
        (:`NewEnumerator0`
          (bind _output_get (set `self.ScanNormailzedTime` (+ (`self.ScanNormailzedTime`) (* (`local.DeltaTime`) (`self.FadeInSpeed`)))))
          (if (>= _output_get 1.0)
            (set `self.ScanNormailzedTime` 1.0)
            (`self.UpdateScanState` "NewEnumerator1")))
        (:`NewEnumerator2`
          (bind _output_get_2 (set `self.ScanNormailzedTime` (- (`self.ScanNormailzedTime`) (* (`local.DeltaTime`) (`self.FadeOutSpeed`)))))
          (if (<= _output_get_2 0.0)
            (set `self.ScanNormailzedTime` 0.0)
            (`self.UpdateScanState` "NewEnumerator3")))
        (:`NewEnumerator4`
          (return false)))
      (`KismetMaterialLibrary.SetScalarParameterValue` null "NormalizedTime" (`self.ScanNormailzedTime`)))
    (:`then_1`
      (return false))))