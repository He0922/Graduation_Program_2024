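; Actor component that drives the player's scan skill, a charged post-process sweep with gathering and burst Niagara effects.
; StartScan and EndScan switch a fade state machine; Tick advances normalized time, starting negative for charge-up, and forces fade-out when energy runs out.
; It feeds time, distance and owner location to MPC_Scan for materials.
; A lazily spawned BP_ScanActor carries the post-process material, with blend weight optionally shaped by a curve.
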(event `self.ReceiveBeginPlay`
  (`self.UpdateScanState` "NewEnumerator3" true)
  (`KismetMaterialLibrary.SetScalarParameterValue` "/Game/VFX/Skill_Material/MPC_Scan.MPC_Scan" "Range" (`self.Range`))
  (`KismetMaterialLibrary.SetScalarParameterValue` "/Game/VFX/Skill_Material/MPC_Scan.MPC_Scan" "GridCellSize" (`self.GridCellSize`)))

(event `self.ReceiveTick`
  (params (DeltaSeconds :type "Float (single-precision)"))
  (bind _returnvalue (`PlayerSkillComponent.GetPlayerNowEnergy` (`self.PlayerSkillComponent`)))
  (if (<= _returnvalue 0.0)
    (`self.UpdateScanState` "NewEnumerator3")
    (else
      (`self.UpdateScanTime` DeltaSeconds)
      (switch `/Game/Character/Skill/Skill_2/Controller/EBP_ScanState` (`self.GetScanState`)
        (:`NewEnumerator0`
          _)
        (:`NewEnumerator2`
          _))
      (`self.UpdateScanPPBlendWeight`)
      (`KismetMaterialLibrary.SetVectorParameterValue` "/Game/VFX/Skill_Material/MPC_Scan.MPC_Scan" "Location" (`KismetMathLibrary.Conv_VectorToLinearColor` (`Actor.K2_GetActorLocation` (`self.GetOwner`)))))))

(fn `DestroyPPActor`
  (bind _scanactor (`self.ScanActor`))
  (if (and (`KismetSystemLibrary.IsValid` _scanactor) (`self.bDestroyActor`))
    (`Actor.K2_DestroyActor` _scanactor)
    (set `self.ScanActor` null)))

(fn `End Scan`
  (switch `/Game/Character/Skill/Skill_2/Controller/EBP_ScanState` (`self.GetScanState`)
    (:`NewEnumerator0`
      _)
    (:`NewEnumerator1`
      _)
    (:`NewEnumerator2`
      (return))
    (:`NewEnumerator3`
      (return))
    (:`NewEnumerator4`
      (return)))
  (`self.UpdateScanState` "NewEnumerator2")
  (`self.Deactivate` (`self.NIagaraComponent`))
  (return))

(fn `GetScanPPActor`
  (returns (`Scan Actor` :type "/Game/Character/Skill/Skill_2/BP_ScanActor Object Reference"))
  (bind _pp_material (`self.PP Material`))
  (bind _postprocess (`/Game/Character/Skill/Skill_2/BP_ScanActor.PostProcess` (`self.ScanActor`)))
  (`/Engine/EditorBlueprintResources/StandardMacros.IsValid` (`self.ScanActor`)
    (:`Is Valid`
      (return (stale _output_get)))
    (:`Is Not Valid`
      (bind _returnvalue (`|SpawnActorFromClass` "/Game/Character/Skill/Skill_2/BP_ScanActor.BP_ScanActor_C" (`KismetMathLibrary.MakeTransform` (0.0 0.0 0.0)) "Undefined" "MultiplyWithRoot" null null))
      (bind _output_get (set `self.ScanActor` _returnvalue))
      (`|ExecutionSequence`
        (:`then_0`
          (`/Engine/EditorBlueprintResources/StandardMacros.IsValid` (`self.PP MID`)
            (:`Is Valid`
              _)
            (:`Is Not Valid`
              (`/Engine/EditorBlueprintResources/StandardMacros.IsValid` _pp_material
                (:`Is Valid`
                  (bind _returnvalue_2 (`KismetMaterialLibrary.CreateDynamicMaterialInstance` _pp_material))
                  (bind _output_get_2 (set `self.PP MID` _returnvalue_2))))))
          (`/Engine/EditorBlueprintResources/StandardMacros.IsValid` _postprocess
            (:`Is Valid`
              (setmembers `PostProcessSettings` :`StructRef` (`PostProcessComponent.Settings` _postprocess) :`AutoExposureMinBrightness` 0.0 :`AutoExposureMaxBrightness` 2.0 :`WeightedBlendables` (make `WeightedBlendables` (`|MakeArray` (make `WeightedBlendable` 1.0 (`self.PP MID`))))))))
        (:`then_1`
          (return _output_get))))))

(fn `GetScanState`
  (returns (State :type "/Game/Character/Skill/Skill_2/Controller/EBP_ScanState Enum"))
  (return (`self.State`)))

(fn `StartScan`
  (params (Distance :type "Float (double-precision)" :default 5000.0) (PSC :type "PlayerSkillComponent Object Reference") (CameraComponent :type "CameraComponent Object Reference"))
  (set `self.CanBurst` true)
  (bind _output_get (set `self.cameraComponent` CameraComponent))
  (set `self.PlayerSkillComponent` PSC)
  (bind _returnvalue (`NiagaraFunctionLibrary.SpawnSystemAttached` (`self.Particle_Gathering`) _output_get "None" (`self.InitPos_Gathering`) (struct) "KeepRelativeOffset"))
  (bind _output_get_2 (set `self.NIagaraComponent` _returnvalue))
  (message `AudioLinkBlueprintInterface.PlayLink` _output_get_2 0.0)
  (set `self.Max Distance` Distance)
  (set `self.ScanNormailzedTime` (- 0.0 (`self.ScanStartTime`)))
  (switch `/Game/Character/Skill/Skill_2/Controller/EBP_ScanState` (`self.GetScanState`)
    (:`NewEnumerator0`
      _)
    (:`NewEnumerator1`
      _)
    (:`NewEnumerator2`
      (`self.UpdateScanState` "NewEnumerator0" :!label _label)
      (return))
    (:`NewEnumerator3`
      (goto _label))
    (:`NewEnumerator4`
      _))
  (return))

(fn `UpdateScanPPBlendWeight`
  (locals (`This Time` :type "Float (single-precision)" :default 0.0))
  (bind _blendcurve (`self.BlendCurve`))
  (bind _scannormailzedtime (`self.ScanNormailzedTime`))
  (`/Engine/EditorBlueprintResources/StandardMacros.IsValid` _blendcurve
    (:`Is Valid`
      (set `local.This Time` (`CurveFloat.GetFloatValue` _blendcurve _scannormailzedtime)))
    (:`Is Not Valid`
      (set `local.This Time` _scannormailzedtime)))
  (bind _scan_actor (`self.GetScanPPActor`))
  (`/Engine/EditorBlueprintResources/StandardMacros.IsValid` _scan_actor
    (:`Is Valid`
      (bind _postprocess (`/Game/Character/Skill/Skill_2/BP_ScanActor.PostProcess` _scan_actor))
      (`/Engine/EditorBlueprintResources/StandardMacros.IsValid` _postprocess
        (:`Is Valid`
          (set `PostProcessComponent.BlendWeight` (`local.This Time`) _postprocess))))))

(fn `UpdateScanState`
  (params (State :type "/Game/Character/Skill/Skill_2/Controller/EBP_ScanState Enum" :default "NewEnumerator0") (Force :type Boolean))
  (returns (Update :type Boolean))
  (if (or Force (`|EnumInequality` State (`self.State`)))
    (`|ExecutionSequence`
      (:`then_0`
        (switch `/Game/Character/Skill/Skill_2/Controller/EBP_ScanState` (`self.State`)
          (:`NewEnumerator1`
            (`KismetMaterialLibrary.SetScalarParameterValue` "/Game/VFX/Skill_Material/MPC_Scan.MPC_Scan" "bFadeIn"))
          (:`NewEnumerator3`
            (`KismetMaterialLibrary.SetScalarParameterValue` "/Game/VFX/Skill_Material/MPC_Scan.MPC_Scan" "bFadeOut")
            (`self.SetComponentTickEnabled` true))))
      (:`then_1`
        (bind _output_get (set `self.State` State))
        (switch `/Game/Character/Skill/Skill_2/Controller/EBP_ScanState` _output_get
          (:`NewEnumerator1`
            (`KismetMaterialLibrary.SetScalarParameterValue` "/Game/VFX/Skill_Material/MPC_Scan.MPC_Scan" "bFadeIn")
            (`self.UpdateScanPPBlendWeight`))
          (:`NewEnumerator3`
            (`KismetMaterialLibrary.SetScalarParameterValue` "/Game/VFX/Skill_Material/MPC_Scan.MPC_Scan" "bFadeOut")
            (`self.UpdateScanPPBlendWeight`)
            (`self.SetComponentTickEnabled` false :!label _label)
            (`self.DestroyPPActor`))
          (:`NewEnumerator4`
            (goto _label))))
      (:`then_2`
        (return true))
      (:`then_3`
        (`KismetSystemLibrary.PrintString` "Update State")))
    (else
      (return false))))

(fn `UpdateScanTime`
  (params (DeltaTime :type "Float (double-precision)"))
  (returns (bUpdated :type Boolean))
  (bind _scannormailzedtime (`self.ScanNormailzedTime`))
  (`|ExecutionSequence`
    (:`then_0`
      (switch `/Game/Character/Skill/Skill_2/Controller/EBP_ScanState` (`self.GetScanState`)
        (:`NewEnumerator0`
          (bind _returnvalue (`KismetMaterialLibrary.GetScalarParameterValue` "/Game/VFX/Skill_Material/MPC_Scan.MPC_Scan" "Complete Charge"))
          (bind _output_get (set `self.ScanNormailzedTime` (+ (`self.ScanNormailzedTime`) (* (`local.DeltaTime`) (select `int` (`KismetMathLibrary.Conv_DoubleToInt64` _returnvalue) :`0` 1.0 :`1` (`self.FadeInSpeed`))))))
          (if (>= _output_get 1.0)
            (set `self.ScanNormailzedTime` 1.0)
            (`self.UpdateScanState` "NewEnumerator1")))
        (:`NewEnumerator2`
          (bind _output_get_2 (set `self.ScanNormailzedTime` (- (`self.ScanNormailzedTime`) (* (`local.DeltaTime`) (`self.FadeOutSpeed`)))))
          (if (<= _output_get_2 0.0)
            (set `self.ScanNormailzedTime` 0.0)
            (`self.UpdateScanState` "NewEnumerator3")))
        (:`NewEnumerator4`
          (return false)))
      (`KismetMaterialLibrary.SetScalarParameterValue` "/Game/VFX/Skill_Material/MPC_Scan.MPC_Scan" "NormalizedTime" _scannormailzedtime)
      (`KismetMaterialLibrary.SetScalarParameterValue` "/Game/VFX/Skill_Material/MPC_Scan.MPC_Scan" "Distance" (* _scannormailzedtime (`self.Max Distance`)))
      (if (<= (`self.ScanNormailzedTime`) -0.1)
        ;[1 1 1] 蓄力中
        (`KismetMaterialLibrary.SetScalarParameterValue` "/Game/VFX/Skill_Material/MPC_Scan.MPC_Scan" "Complete Charge")
        (else
          ;[1 1 1] 蓄力完成
          (`KismetMaterialLibrary.SetScalarParameterValue` "/Game/VFX/Skill_Material/MPC_Scan.MPC_Scan" "Complete Charge" 1.0))))
    (:`then_1`
      (if (and (>= (`self.ScanNormailzedTime`) (`self.BurstStartTime`)) (`self.CanBurst`))
        (`SceneComponent.K2_AddLocalOffset` (`self.NiagaraComponent`) (`self.InitPos_Burst`) false false)
        (`NiagaraComponent.SetAsset` (`self.NiagaraComponent`) (`self.Particle_Burst`) true)
        (message `AudioLinkBlueprintInterface.PlayLink` (`self.NiagaraComponent`) 0.0)
        (set `self.CanBurst` false)))
    (:`then_2`
      (return false))))