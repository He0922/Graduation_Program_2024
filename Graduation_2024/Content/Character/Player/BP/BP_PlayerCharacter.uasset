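; Player character Blueprint that handles the scan ability input.
; Pressing IA_Scan checks for a controller, a BP_ScanController component and no scan cooldown, then starts a scan using the skill component's distance and the camera.
; Releasing the input ends the scan.
; The event graph holds only empty events and disconnected debug prints for player status, capsule collision and unlocked archival points.
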(event `self.ReceiveBeginPlay`)

(event `self.ReceiveTick`
  (params (DeltaSeconds :type "Float (single-precision)")))

(event `EnhancedInput|/Game/Character/Player/EnhancedInput/Character_InputAction/IA_Scan`
  (params (ActionValue :type Boolean) (ElapsedSeconds :type "Float (double-precision)") (TriggeredSeconds :type "Float (double-precision)") (InputAction :type "InputAction Object Reference" :default "/Game/Character/Player/EnhancedInput/Character_InputAction/IA_Scan.IA_Scan"))
  (bind _playerskillcomponent (`self.playerSkillComponent`))
  (bind _returnvalue (`self.GetComponentByClass` self "/Game/Character/Skill/Skill_2/Controller/BP_ScanController.BP_ScanController_C"))
  (bind _returnvalue_2 (`self.GetComponentByClass` self "/Game/Character/Skill/Skill_2/Controller/BP_ScanController.BP_ScanController_C"))
  (:`Started`
    (`/Engine/EditorBlueprintResources/StandardMacros.IsValid` (`self.GetController`)
      (:`Is Valid`
        (`/Engine/EditorBlueprintResources/StandardMacros.IsValid` _returnvalue_2
          (:`Is Valid`
            (if (not (`PlayerSkillComponent.GetScanColdState` _playerskillcomponent))
              (`/Game/Character/Skill/Skill_2/Controller/BP_ScanController.StartScan` _returnvalue_2 (`PlayerSkillComponent.GetScanDistance` _playerskillcomponent) _playerskillcomponent (`self.camera`))
              (`KismetSystemLibrary.PrintString` "Start Scan")))))))
  (:`Completed`
    (`/Engine/EditorBlueprintResources/StandardMacros.IsValid` (`self.GetController`)
      (:`Is Valid`
        (`/Engine/EditorBlueprintResources/StandardMacros.IsValid` _returnvalue
          (:`Is Valid`
            (`/Game/Character/Skill/Skill_2/Controller/BP_ScanController.End Scan` _returnvalue)
            (`KismetSystemLibrary.PrintString` "End Scan")))))))

(fn `UserConstructionScript`)